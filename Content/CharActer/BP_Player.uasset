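; Player character Blueprint that grants sprint, skill attack and capture actions and drives a HUD widget for health and cooldowns.
; A test input starts a cooldown countdown and spawns a HandActor projectile, which a looping timer steers along the view direction while its override flag is set.
; Helper functions sample trace points along the weapon socket and compute curved paths by rotating interpolated offsets, previewed with debug spheres in a test event.
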(event Custom|tests
  (bind (_outlocation _outrotation) (Actor|GetActorEyesViewPoint))
  (if (Variables|/Game/CharActer/HandActor.HandActor_C|GetisOverride (stale Input|ActionEvents|InputActiontest _returnvalue_2))
    (if (Variables|/Game/CharActer/HandActor.HandActor_C|GetisDestroy (stale Input|ActionEvents|InputActiontest _returnvalue_2))
      (Utilities|Time|ClearandInvalidateTimerbyHandle (Variables|Default|GetTimerHandle))
      (else
        (Variables|/Script/Engine.MovementComponent|SetVelocity (Variables|/Game/CharActer/HandActor.HandActor_C|GetProjectileMovement (stale Input|ActionEvents|InputActiontest _returnvalue_2)) (- (+ (* (Math|Vector|GetForwardVector _outrotation) (Math|Vector|VectorLength (- (Transformation|GetActorLocation (stale Input|ActionEvents|InputActiontest _returnvalue_2)) _outlocation))) _outlocation) (Transformation|GetActorLocation (stale Input|ActionEvents|InputActiontest _returnvalue_2))))))))

(event Custom|HealthChanged
  (params (InstigatorActor :type Actor%20Object%20Reference) (OwningComp :type S%20Attribute%20Component%20Object%20Reference) (NewHealth :type Float%20%28single-precision%29) (Delta :type Float%20%28single-precision%29) (HitLocation :type Vector))
  (bind _wb_harm (Variables|Default|GetWB_Harm))
  (Utilities|IsValid _wb_harm
    (:Is%20Valid
      (Default|UpdateHealth _wb_harm InstigatorActor OwningComp NewHealth Delta HitLocation))))

(event Custom|SetCD2
  (params (value :type Integer))
  (Default|SetCD2 (Variables|Default|GetWB_Harm) value))

(event Custom|SetCD1
  (params (value :type Integer))
  (Default|SetCD (Variables|Default|GetWB_Harm) value))

(event Custom|SetCD3
  (Default|SetCD3 (Variables|Default|GetWB_Harm) (Variables|Default|GetCD3V))
  (bind _result (Math|Integer|DecrementInt (Variables|Default|GetCD3V))
    (:%20%20
      (bind _output_get (Variables|Default|SetCD3V _result))
      (if (== _output_get -1)
        (Utilities|Time|ClearandInvalidateTimerbyHandle (Variables|Default|GetTimerCD))
        (Variables|Default|SetCD3V 5)))))

(event Custom|test
  (Utilities|FlowControl|DoOnce false ; enters at Reset
    (:Completed
      (bind _returnvalue (Actor|GetActorOfClass "/Game/AI/NewBlueprint.NewBlueprint_C"))
      (bind _resultlocation (CallFunction|CalculateLocation (Transformation|GetActorLocation _returnvalue) (Transformation|GetActorForwardVector _returnvalue) (Transformation|GetActorLocation) 5))
      (bind _output_get (Variables|Default|SetCurrent%20Attack%20Point _resultlocation))
      (for _array_element _output_get
        (Rendering|Debug|DrawDebugSphere _array_element 1e+01 12 "(R=1.000000,G=0.122771,B=0.182505,A=1.000000)" 2.0 2.0))
      (CallFunction|Test))))

(event EventBeginPlay
  (bind _actioncomp (Variables|Default|GetActionComp))
  (bind _returnvalue (UserInterface|CreateWidget "/Game/UI/WB_Health.WB_Health_C" 0 (Variables|Default|GetHandActor)))
  (bind _output_get (Variables|Default|SetWB_Harm _returnvalue))
  (EventDispatchers|BindEventtoOnHealthChanged (Variables|Default|GetAttributeComponent) (delegate Custom|HealthChanged))
  (UserInterface|Viewport|AddtoViewport _output_get 0)
  (EventDispatchers|BindEventtoCD1 (delegate Custom|SetCD1))
  (EventDispatchers|BindEventtoCD2 (delegate Custom|SetCD2))
  (Class|SActionComponent|AddAction _actioncomp "/Game/CharActer/Actions/BP_ActionSprint.BP_ActionSprint_C")
  (Class|SActionComponent|AddAction _actioncomp "/Game/CharActer/BP_SkillAttack.BP_SkillAttack_C")
  (Class|SActionComponent|AddAction _actioncomp "/Game/CharActer/Actions/BP_ActionCapture.BP_ActionCapture_C"))

(event EventTick
  (params (DeltaSeconds :type Float%20%28single-precision%29)))

(event Input|ActionEvents|InputActiontest
  (params (Key :type Key%20Structure :default "None"))
  (bind (_outlocation _outrotation) (Actor|GetActorEyesViewPoint))
  (:Pressed
    (if (not (Utilities|Time|IsValidTimerHandle (Variables|Default|GetTimerCD)))
      (bind _returnvalue (Utilities|Time|SetTimerbyEvent (delegate Custom|SetCD3) 1.0 true))
      (Variables|Default|SetTimerCD _returnvalue)
      (bind _returnvalue_2 (Game|SpawnActorfromClass "/Game/CharActer/HandActor.HandActor_C" (Math|Transform|MakeTransform (+ _outlocation (* (Math|Vector|GetForwardVector _outrotation) 1e+02)) _outrotation "1.000000,1.000000,1.000000") "Undefined" "MultiplyWithRoot" 0 0))
      (bind _returnvalue_3 (Utilities|Time|SetTimerbyEvent (delegate Custom|tests) 0.2 true))
      (Variables|Default|SetTimerHandle _returnvalue_3))))

(fn ConstructionScript)

(fn GetAttackTracePoint
  (bind _mesh (Variables|Character|GetMesh))
  (for _index (range 0 4)
    (Utilities|Array|SetArrayElem (Variables|Default|GetAttack%20Point) _index (+ (Transformation|GetSocketLocation _mesh "Weapon_02") (* _index (* (Math|Vector|GetForwardVector (Transformation|GetSocketRotation _mesh "Weapon_02")) 25.0))) true))
  (return (Variables|Default|GetAttack%20Point)))

(fn CalculateLocation
  (params (StartLocation :type Vector) (ForwardLocation :type Vector) (EndLocation :type Vector) (Count :type Integer))
  (bind _returnvalue (Math|Vector|GetUnitDirection(Vector) StartLocation EndLocation))
  (bind _returnvalue_2 (Math|Vector|CrossProduct _returnvalue ForwardLocation))
  (bind _output_get (LocalVariables|SetMeanLocation (/ (- EndLocation StartLocation) Count)))
  (for _index (range 0 Count)
    (Utilities|Array|Add (LocalVariables|GetResultLocations) (+ StartLocation (Math|Vector|RotateVectorAroundAxis (* _output_get _index) (* (- Count _index) (/ (* (Class|KismetMathLibrary|DegAcos (Class|KismetMathLibrary|VectorCosineAngle2D ForwardLocation _returnvalue)) (/ (.z _returnvalue_2) (Math|Float|Absolute(Float) (.z _returnvalue_2)))) Count)) "0.000000,0.000000,1.000000"))))
  (return (LocalVariables|GetResultLocations)))